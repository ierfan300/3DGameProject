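; CanonBP is a hazard actor that damages the third-person player character on contact with its collision sphere.
; Each overlap with BP_ThirdPersonCharacter plays a 2D sound and subtracts a fixed amount directly from the character's HealthValue.
; When health reaches zero or below, the hazard itself creates the GameOver_WBP widget, shows the mouse cursor and pauses the game.
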(event `self.SphereCollision.OnComponentBeginOverlap`
  (params (OverlappedComponent :type "PrimitiveComponent Object Reference") (OtherActor :type "Actor Object Reference") (OtherComp :type "PrimitiveComponent Object Reference") (OtherBodyIndex :type Integer) (bFromSweep :type Boolean) (SweepResult :type "HitResult Structure (by ref)"))
  (bind _asbp_third_person_character (cast `/Game/ThirdPerson/Blueprints/BP_ThirdPersonCharacter` OtherActor))
  (`GameplayStatics.PlaySound2D` "/Engine/EditorSounds/GamePreview/EjectFromPlayer.EjectFromPlayer" 1.0 1.0 0.0 null null)
  (bind _healthvalue (`/Game/ThirdPerson/Blueprints/BP_ThirdPersonCharacter.HealthValue` _asbp_third_person_character))
  (set `/Game/ThirdPerson/Blueprints/BP_ThirdPersonCharacter.HealthValue` (- _healthvalue 10.0) _asbp_third_person_character)
  (if (<= _healthvalue 0.0)
    (bind _returnvalue (`|CreateWidget` "/Game/ActorBP/GameOver_WBP.GameOver_WBP_C"))
    (`UserWidget.AddToViewport` _returnvalue 0)
    (set `PlayerController.bShowMouseCursor` true (`GameplayStatics.GetPlayerController` 0))
    (`GameplayStatics.SetGamePaused` true)))

(fn `UserConstructionScript`)