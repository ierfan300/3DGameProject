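; Collectible item actor that the third-person character picks up by walking into it.
; Overlapping its sphere increments that character's Pickup count, plays a 2D sound and destroys the item.
; Once the count reaches two or more, it sets ItemNumberReached on the first player's character.
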(event `self.Sphere1.OnComponentBeginOverlap`
  (params (OverlappedComponent :type "PrimitiveComponent Object Reference") (OtherActor :type "Actor Object Reference") (OtherComp :type "PrimitiveComponent Object Reference") (OtherBodyIndex :type Integer) (bFromSweep :type Boolean) (SweepResult :type "HitResult Structure (by ref)"))
  (bind _asbp_third_person_character (cast `/Game/ThirdPerson/Blueprints/BP_ThirdPersonCharacter` OtherActor))
  (bind _pickup (`/Game/ThirdPerson/Blueprints/BP_ThirdPersonCharacter.Pickup` _asbp_third_person_character))
  (set `/Game/ThirdPerson/Blueprints/BP_ThirdPersonCharacter.Pickup` (+ _pickup 1) _asbp_third_person_character)
  (`GameplayStatics.PlaySound2D` "/Engine/EditorSounds/Notifications/CompileFailed_Cue.CompileFailed_Cue" 1.0 1.0 0.0 null null)
  (`self.K2_DestroyActor`)
  (if (>= _pickup 2)
    (bind _asbp_third_person_character_2 (cast `/Game/ThirdPerson/Blueprints/BP_ThirdPersonCharacter` (`GameplayStatics.GetPlayerCharacter` 0)))
    (set `/Game/ThirdPerson/Blueprints/BP_ThirdPersonCharacter.ItemNumberReached` true _asbp_third_person_character_2)))

(fn `UserConstructionScript`)